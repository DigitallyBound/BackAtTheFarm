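; Buck is a collectable money pickup that increments the player's BucksCount on overlap.
; On spawn a collectable buck gets a random upward physics impulse with a coin sound, then spins each tick.
; When a SIM_Player touches its trigger, it disables physics and collision, plays a cash sound, then rises while spinning until a timer destroys it two seconds later.
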(event `self.ReceiveTick`
  (params (DeltaSeconds :type "Float (single-precision)"))
  (bind _buck_mesh (`self.Buck_Mesh`))
  ;[1 1 1] Tick Event
  (if (`self.isCollectable`)
    (`SceneComponent.K2_AddLocalRotation` _buck_mesh (`KismetMathLibrary.MakeRotator` (.roll (`self.K2_GetActorRotation`)) (.pitch (`self.K2_GetActorRotation`)) (+ (.yaw (`self.K2_GetActorRotation`)) 1.0)) false false)
    (else
      (`SceneComponent.K2_AddLocalRotation` _buck_mesh (struct :`Yaw` 10.0) false false)
      (`SceneComponent.K2_AddLocalOffset` (`self.Buck_Mesh`) (0.0 0.0 5.0) false false))))

(event `self.ReceiveBeginPlay`
  (bind _buck_mesh (`self.Buck_Mesh`))
  ;[1 1 1] Start
  (if (`self.isCollectable`)
    (`PrimitiveComponent.AddImpulse` _buck_mesh (`KismetMathLibrary.MakeVector` (`KismetMathLibrary.RandomFloatInRange` -250.0 250.0) (`KismetMathLibrary.RandomFloatInRange` -250.0 250.0) 500.0) "None" true)
    (`GameplayStatics.PlaySoundAtLocation` "/Game/Audio/Effects/coin01.coin01" (`SceneComponent.K2_GetComponentLocation` _buck_mesh) (struct) 0.6 1.0 0.0 null null null)))

(event `self.Trigger.OnComponentBeginOverlap`
  (params (OverlappedComponent :type "PrimitiveComponent Object Reference") (OtherActor :type "Actor Object Reference") (OtherComp :type "PrimitiveComponent Object Reference") (OtherBodyIndex :type Integer) (bFromSweep :type Boolean) (SweepResult :type "HitResult Structure (by ref)"))
  (bind _buck_mesh (`self.Buck_Mesh`))
  ;[1 1 1] Player Collision
  (if (`self.isCollectable`)
    (bind _assim_player (cast `/Game/OldPrototype/Blueprints/SIM_Player` OtherActor))
    (set `/Game/OldPrototype/Blueprints/SIM_Player.Bucks Count` (+ (`/Game/OldPrototype/Blueprints/SIM_Player.Bucks Count` _assim_player) 1) _assim_player)
    (set `self.isCollectable` false)
    (`PrimitiveComponent.SetSimulatePhysics` _buck_mesh false)
    (`PrimitiveComponent.SetCollisionEnabled` _buck_mesh "NoCollision")
    (`KismetSystemLibrary.K2_SetTimerDelegate` (delegate `Destruct`) 2.0)
    (`GameplayStatics.PlaySound2D` "/Game/Audio/Effects/cash.cash" 1.0 1.0 0.0 null null)))

(event `Destruct`
  ;[1 1 1] Destruct Event
  (`self.K2_DestroyActor`))

(fn `UserConstructionScript`)