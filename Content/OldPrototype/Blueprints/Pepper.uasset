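; Collectable pepper pickup that refills a SIM_Player's stamina on touch.
; While collectable, the mesh spins, and on BeginPlay it is launched upward with a random sideways impulse.
; On overlap it sets the player's stamina and pepper timing variables, turns off mesh physics and collision, and plays a sizzle sound.
; The collected pepper then spins faster and rises until a timer destroys the actor.
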(event `self.ReceiveTick`
  (params (DeltaSeconds :type "Float (single-precision)"))
  (bind _pepper_mesh (`self.Pepper_Mesh`))
  ;[1 1 1] Tick Event
  (if (`self.isCollectable`)
    (`SceneComponent.K2_AddLocalRotation` _pepper_mesh (`KismetMathLibrary.MakeRotator` (.roll (`self.K2_GetActorRotation`)) (.pitch (`self.K2_GetActorRotation`)) (+ (.yaw (`self.K2_GetActorRotation`)) 1.0)) false false)
    (else
      (`SceneComponent.K2_AddLocalRotation` _pepper_mesh (struct :`Yaw` 10.0) false false)
      (`SceneComponent.K2_AddLocalOffset` (`self.Pepper_Mesh`) (0.0 0.0 5.0) false false))))

(event `self.ReceiveBeginPlay`
  ;[1 1 1] Start
  (if (`self.isCollectable`)
    (`PrimitiveComponent.AddImpulse` (`self.Pepper_Mesh`) (`KismetMathLibrary.MakeVector` (`KismetMathLibrary.RandomFloatInRange` -250.0 250.0) (`KismetMathLibrary.RandomFloatInRange` -250.0 250.0) 500.0) "None" true)))

(event `self.Trigger.OnComponentBeginOverlap`
  (params (OverlappedComponent :type "PrimitiveComponent Object Reference") (OtherActor :type "Actor Object Reference") (OtherComp :type "PrimitiveComponent Object Reference") (OtherBodyIndex :type Integer) (bFromSweep :type Boolean) (SweepResult :type "HitResult Structure (by ref)"))
  (bind _pepper_mesh (`self.Pepper_Mesh`))
  ;[1 1 1] Player Collision
  (if (`self.isCollectable`)
    (bind _assim_player (cast `/Game/OldPrototype/Blueprints/SIM_Player` OtherActor))
    (bind _output_get (set `/Game/OldPrototype/Blueprints/SIM_Player.Stamina` (`/Game/OldPrototype/Blueprints/SIM_Player.MaxStamina` _assim_player) _assim_player))
    (`|ExecutionSequence`
      (:`then_0`
        (`/Game/OldPrototype/Blueprints/SIM_Player.GetPrecisionFloat` _assim_player _output_get 1)
        (set `/Game/OldPrototype/Blueprints/SIM_Player.LastStaminaResetTime` 5.0 _assim_player)
        (set `self.isCollectable` false)
        (`PrimitiveComponent.SetSimulatePhysics` _pepper_mesh false)
        (`PrimitiveComponent.SetCollisionEnabled` _pepper_mesh "NoCollision")
        (`KismetSystemLibrary.K2_SetTimerDelegate` (delegate `Destruct`) 2.0)
        (`GameplayStatics.PlaySound2D` "/Game/Audio/Effects/sizzle.sizzle" 0.4 1.0 0.0 null null))
      (:`then_1`
        (set `/Game/OldPrototype/Blueprints/SIM_Player.LastPepperTime` 0.0 _assim_player)))))

(event `Destruct`
  ;[1 1 1] Destruct Event
  (`self.K2_DestroyActor`))

(fn `UserConstructionScript`)