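; Prototype AI controller that makes its NPC pawn wander continuously.
; After a short delay it moves to a random reachable point around the pawn's current location, then repeats whether the move succeeds or fails.
; Every tick, while the TestNPC pawn's BlockMovement flag is set, it issues an AIMoveTo targeting the controller itself, apparently to override wandering.
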(event `self.ReceiveBeginPlay`
  (`KismetSystemLibrary.Delay` 0.2 :!label _label)
  (`self.GoToLocation` (`self.K2_GetActorLocation` (`self.K2_GetPawn`))))

(event `self.ReceiveTick`
  (params (DeltaSeconds :type "Float (single-precision)"))
  (bind _astest_npc (cast `/Game/OldPrototype/Blueprints/AI/TestNPC` (`self.K2_GetPawn`)))
  (if (`/Game/OldPrototype/Blueprints/AI/TestNPC.BlockMovement` _astest_npc)
    (`|AIMoveTo` null (0.0 0.0 0.0) self)))

(event `self.GoToLocation`
  (params (TargetLocation :type "Vector Structure"))
  (`|AIMoveTo` null (`NavigationSystemV1.K2_GetRandomReachablePointInRadius` TargetLocation 1000.0 null null) null 150.0 true
    (:`OnSuccess`
      (goto _label))
    (:`OnFail`
      (goto _label))))

(fn `UserConstructionScript`)