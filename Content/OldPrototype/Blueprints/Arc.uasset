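; Arc is a rotating level-entrance marker that takes the player to the level named by LevelName.
; Its trigger overlap toggles an active flag and the ENTER_BARN center text on the player's HUD.
; Pressing Interact while active saves through the player pawn, then opens the level.
; Tick spins the arc, with the arrow turning faster; a vertical arrow bobbing timeline exists but never runs.
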(event `InputAction|Interact` :consume false
  (params (Key :type "Key Structure"))
  ;[1 1 1] Interact
  (:`Pressed`
    (if (`self.IsActive`)
      (bind _assim_player (cast `` (`GameplayStatics.GetPlayerPawn` 0)))
      (`self.Save` _assim_player)
      (`GameplayStatics.OpenLevel` (`self.Level Name`)))))

(event `self.ReceiveTick`
  (params (DeltaSeconds :type "Float (single-precision)"))
  (bind _returnvalue (* DeltaSeconds 40.0))
  ;[1 1 1] Loop
  (`SceneComponent.K2_AddLocalRotation` (`self.Arc`) (`KismetMathLibrary.MakeRotator` 0.0 0.0 _returnvalue) false false)
  (`SceneComponent.K2_AddLocalRotation` (`self.Arrow`) (`KismetMathLibrary.MakeRotator` 0.0 0.0 (* _returnvalue 4.0)) false false))

(event `self.Trigger.OnComponentBeginOverlap`
  (params (OverlappedComponent :type "PrimitiveComponent Object Reference") (OtherActor :type "Actor Object Reference") (OtherComp :type "PrimitiveComponent Object Reference") (OtherBodyIndex :type Integer) (bFromSweep :type Boolean) (SweepResult :type "HitResult Structure (by ref)"))
  ;[1 1 1] HUD Info
  (cast `` OtherActor)
  (set `self.isPlayerIn` true)
  (bind _assim_player (cast `` (`GameplayStatics.GetPlayerPawn` 0) :!label _label))
  (if (`self.isPlayerIn`)
    (bind _hud (`/Game/OldPrototype/Blueprints/Arc.HUD` _assim_player))
    (set `/Game/OldPrototype/Blueprints/Arc.Center_Text` "ENTER_BARN" _hud)
    (set `self.isActive` true)
    (else
      (set `/Game/OldPrototype/Blueprints/Arc.Center_Text` "" _hud)
      (set `self.isActive` false))))

(event `self.Trigger.OnComponentEndOverlap`
  (params (OverlappedComponent :type "PrimitiveComponent Object Reference") (OtherActor :type "Actor Object Reference") (OtherComp :type "PrimitiveComponent Object Reference") (OtherBodyIndex :type Integer))
  ;[1 1 1] HUD Info
  (cast `` OtherActor)
  (set `self.isPlayerIn` false)
  (goto _label))

(fn `UserConstructionScript`)