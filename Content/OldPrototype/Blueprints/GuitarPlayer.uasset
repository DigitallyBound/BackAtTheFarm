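; Player Blueprint for a guitar prototype that plays one of six chords (C, E, F, G, Dm, Am) from WASD and the two mouse buttons.
; Each press picks a chord sound, replaces any playing audio component with one spawned at the actor's location, and highlights the chord on a Chords HUD widget created at BeginPlay.
; An audio-finished binding clears the highlight, and unbinding before destroying the old sound keeps interruptions from clearing it.
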(event `Key|RightMouseButton`
  (params (Key :type "Key Structure"))
  (:`Pressed`
    (set `self.Chord` "/Game/Audio/Chords/f.f")
    (`self.Play_Guitar`)
    (`self.SetActiveChord` 1)))

(event `Key|LeftMouseButton`
  (params (Key :type "Key Structure"))
  (:`Pressed`
    (set `self.Chord` "/Game/Audio/Chords/am.am")
    (`self.Play_Guitar`)
    (`self.SetActiveChord` 5)))

(event `Key|A`
  (params (Key :type "Key Structure"))
  (:`Pressed`
    (set `self.Chord` "/Game/Audio/Chords/dm.dm")
    (`self.Play_Guitar`)
    (`self.SetActiveChord` 4)))

(event `Key|D`
  (params (Key :type "Key Structure"))
  (:`Pressed`
    (set `self.Chord` "/Game/Audio/Chords/e.e")
    (`self.Play_Guitar`)
    (`self.SetActiveChord` 2)))

(event `Key|W`
  (params (Key :type "Key Structure"))
  (:`Pressed`
    (set `self.Chord` "/Game/Audio/Chords/c.c")
    (`self.Play_Guitar`)
    (`self.SetActiveChord` 0)))

(event `Key|S`
  (params (Key :type "Key Structure"))
  (:`Pressed`
    (set `self.Chord` "/Game/Audio/Chords/g.g")
    (`self.Play_Guitar`)
    (`self.SetActiveChord` 3)))

(event `self.ReceiveBeginPlay`
  (bind _returnvalue (`|CreateWidget` "/Game/OldPrototype/Blueprints/GameModes/Guitar/Chords.Chords_C" (`GameplayStatics.GetPlayerController` 0)))
  (bind _output_get (set `self.ChordsHUD` _returnvalue))
  (`UserWidget.AddToViewport` _output_get 0))

(event `Play_Guitar`
  (bind (_returnvalue_location _returnvalue_rotation) (`KismetMathLibrary.BreakTransform` (`self.GetTransform` self)))
  (bind _audiocomponent (`self.AudioComponent`)
    (:`then`
      (clear `AudioComponent.OnAudioFinished` _audiocomponent)
      (`ActorComponent.K2_DestroyComponent` _audiocomponent))
    (:`else`
      _))
  (bind _returnvalue (`GameplayStatics.SpawnSoundAtLocation` (`self.Chord`) _returnvalue_location _returnvalue_rotation 1.0 1.0 0.0 null null))
  (bind _output_get (set `self.AudioComponent` _returnvalue))
  (add `AudioComponent.OnAudioFinished` _output_get (delegate `Reset Chord`)))

(event `Reset Chord`
  (`self.SetActiveChord` -1))

(event `SetActiveChord`
  (params (ChordNum :type Integer))
  (`/Game/OldPrototype/Blueprints/GameModes/Guitar/Chords.SetChord` (`self.ChordsHUD`) ChordNum))

(fn `UserConstructionScript`)