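; Milk is a thrown projectile actor that marks players and NPCs it touches as milked.
; On spawn, impulses launch its Sphere along the owner's forward vector with an upward arc, and it self-destructs after a short delay or on any hit.
; Overlaps ignore the instigator and other Milk, setting IsMilked and calling PlanClean on an unmilked SIM_Player or TestNPC; all other overlaps just destroy it.
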(event `self.ReceiveBeginPlay`
  (bind _sphere (`self.Sphere`))
  (`PrimitiveComponent.AddImpulse` _sphere (* (`self.GetActorForwardVector` (`self.GetOwner`)) 1200.0) "None" true)
  (`PrimitiveComponent.AddImpulse` _sphere (0.0 0.0 400.0) "None" true)
  (`KismetSystemLibrary.Delay` 5.0)
  (`self.K2_DestroyActor`))

(event `self.Sphere.OnComponentHit`
  (params (HitComponent :type "PrimitiveComponent Object Reference") (OtherActor :type "Actor Object Reference") (OtherComp :type "PrimitiveComponent Object Reference") (NormalImpulse :type "Vector Structure") (Hit :type "HitResult Structure (by ref)"))
  (`self.K2_DestroyActor` :!label _label))

(event `self.Sphere.OnComponentBeginOverlap`
  (params (OverlappedComponent :type "PrimitiveComponent Object Reference") (OtherActor :type "Actor Object Reference") (OtherComp :type "PrimitiveComponent Object Reference") (OtherBodyIndex :type Integer) (bFromSweep :type Boolean) (SweepResult :type "HitResult Structure (by ref)"))
  (if (and (!= (`self.GetInstigator`) OtherActor) (!= (`GameplayStatics.GetObjectClass` OtherActor) "Milk_C"))
    (bind _assim_player (cast `/Game/OldPrototype/Blueprints/SIM_Player` OtherActor)
      (:`then`
        (if (`/Game/OldPrototype/Blueprints/SIM_Player.isMilked` _assim_player)
          (`self.K2_DestroyActor` :!label _label_2)
          (else
            (set `/Game/OldPrototype/Blueprints/SIM_Player.isMilked` true _assim_player)
            (`self.K2_DestroyActor`)
            (`/Game/OldPrototype/Blueprints/SIM_Player.PlanClean` _assim_player))))
      (:`CastFailed`
        (bind _astest_npc (cast `/Game/OldPrototype/Blueprints/AI/TestNPC` OtherActor)
          (:`then`
            (if (`/Game/OldPrototype/Blueprints/AI/TestNPC.isMilked` _astest_npc)
              (goto _label)
              (else
                (set `/Game/OldPrototype/Blueprints/AI/TestNPC.isMilked` true _astest_npc)
                (`self.K2_DestroyActor`)
                (`/Game/OldPrototype/Blueprints/AI/TestNPC.PlanClean` _astest_npc))))
          (:`CastFailed`
            (goto _label_2)))))))

(fn `UserConstructionScript`)