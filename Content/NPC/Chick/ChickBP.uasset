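; ChickBP is a chick NPC that wanders and reacts when the player overlaps its trigger.
; On Tick, while neither moving nor stopped, it starts an AI move to a random reachable nearby point, and the IsMoving flag clears on success or failure so wandering repeats.
; When an empty-handed ThirdPersonCharacter enters Trigger, it adds a child actor component.
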(event `self.ReceiveTick`
  (params (DeltaSeconds :type "Float (single-precision)"))
  (if (and (not (`self.isMoving`)) (not (`self.Stopped`)))
    (set `self.isMoving` true)
    (`|AIMoveTo` self (`NavigationSystemV1.K2_GetRandomReachablePointInRadius` (`self.K2_GetActorLocation`) 500.0 null null) null 50.0 true
      (:`OnSuccess`
        _)
      (:`OnFail`
        _))
    (set `self.isMoving` false)))

(event `self.Trigger.OnComponentBeginOverlap`
  (params (OverlappedComponent :type "PrimitiveComponent Object Reference") (OtherActor :type "Actor Object Reference") (OtherComp :type "PrimitiveComponent Object Reference") (OtherBodyIndex :type Integer) (bFromSweep :type Boolean) (SweepResult :type "HitResult Structure (by ref)"))
  (bind _asthird_person_character (cast `/Game/ThirdPersonBP/Blueprints/ThirdPersonCharacter` OtherActor))
  (if (not (`/Game/ThirdPersonBP/Blueprints/ThirdPersonCharacter.HaveItemInHand` _asthird_person_character))
    (`AddComponent|NODE_AddChildActorComponent-0`)))

(fn `UserConstructionScript`)